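; BP_HexGrid is a prototype hex grid actor that builds tile maps in rhombus, hexagon or rectangle shapes.
; Each generate event cleans up the existing grid, builds a map from its shape parameters and passes it to InitializeHexGrid.
; On BeginPlay it creates WB_HexTileTest with a reference to itself, caches it and adds it to the viewport as a test UI.
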(event Custom|ShowTestWidget
  (Utilities|IsValid (Variables|Default|GetTestWidget)
    (:Is%20Valid
      (UserInterface|Viewport|AddtoViewport (Variables|Default|GetTestWidget) 0))
    (:Is%20Not%20Valid
      (bind _returnvalue (UserInterface|CreateWidget "/Game/_PROTO/WB_HexTileTest.WB_HexTileTest_C" (Game|GetPlayerController 0) self))
      (bind _output_get (Variables|Default|SetTestWidget _returnvalue))
      (UserInterface|Viewport|AddtoViewport _output_get 0))))

(event Custom|GenerateHex
  (params (Spread :type Integer))
  (CallFunction|Cleanup)
  (bind _returnvalue (Class|BasicHexBlueprintFunctionLibrary|GenerateHexMap Spread))
  (Class|HexGridActor|InitializeHexGrid _returnvalue))

(event Custom|Cleanup
  (Class|HexGridActor|CleanupHexGrid))

(event Custom|GenerateRhombus
  (params (NumRows :type Integer) (RowLength :type Integer))
  (CallFunction|Cleanup)
  (bind _returnvalue (Class|BasicHexBlueprintFunctionLibrary|GenerateRhombusMap NumRows RowLength))
  (Class|HexGridActor|InitializeHexGrid _returnvalue))

(event Custom|GenerateRectangle
  (params (left :type Integer) (right :type Integer) (top :type Integer) (bottom :type Integer))
  (CallFunction|Cleanup)
  (bind _returnvalue (Class|BasicHexBlueprintFunctionLibrary|GenerateRectangleMap left right top bottom))
  (Class|HexGridActor|InitializeHexGrid _returnvalue))

(event EventBeginPlay
  (CallFunction|ShowTestWidget))

(fn ConstructionScript)