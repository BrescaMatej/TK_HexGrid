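; Prototype player pawn whose orthographic camera follows and frames a BP_HexTile actor, with input hooks for hex tests.
; A looping timer polls for the first tile, stops once found and restarts when that tile is destroyed.
; Tick smoothly interpolates location and ortho width to the tile mesh's bounds.
; Left click traces vertically under the cursor to remove the closest instanced mesh instance; Space prints a Hex addition operator test.
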(event Custom|SlowTickEvent
  ;[0 0 0] Slow tick waiting wor hex tile actor to be spawned in the world for use with the normal  tick
  (bind _outactors (Actor|GetAllActorsOfClass "/Game/_PROTO/BP_HexTile.BP_HexTile_C"))
  (if (Utilities|Array|IsEmpty _outactors)
    (Variables|Default|SetHexTileActor 0)
    (else
      (bind _output_get (Variables|Default|SetHexTileActor (Utilities|Array|Get(acopy) _outactors)))
      (Game|AssignOnDestroyed _output_get (delegate Custom|OnFocusTileActorDestroyed))
      (Utilities|Time|ClearandInvalidateTimerbyHandle (Variables|Default|GetSlowTickTimer)))))

(event Custom|StartSlowTick
  ;[0 0 0] Slow tick waiting wor hex tile actor to be spawned in the world for use with the normal  tick
  (bind _returnvalue (Utilities|Time|SetTimerbyEvent (delegate Custom|SlowTickEvent) 0.1 true))
  (Variables|Default|SetSlowTickTimer _returnvalue))

(event Custom|OnFocusTileActorDestroyed
  (params (DestroyedActor :type Actor%20Object%20Reference))
  ;[0 0 0] Slow tick waiting wor hex tile actor to be spawned in the world for use with the normal  tick
  (CallFunction|StartSlowTick))

(event Custom|TickCameraUpdate
  (params (Delta :type Float%20%28double-precision%29))
  (bind _hextileactor (Variables|Default|GetHexTileActor))
  (bind _camera (Variables|Default|GetCamera))
  (bind _hex_tile_instanced_mesh (Default|GetHexTileMesh _hextileactor))
  (bind (_origin _boxextent) (Collision|GetComponentBounds _hex_tile_instanced_mesh))
  (bind (_x _y) (Math|Vector|BreakVector _boxextent))
  ;[1 0 0] Coemstic camera update tick event
  (Utilities|IsValid _hextileactor
    (:Is%20Valid
      (Transformation|SetActorLocation (Math|Interpolation|VInterpTo (Transformation|GetActorLocation) _origin Delta 2.0) false false)
      (Class|CameraComponent|SetOrthoWidth _camera (Math|Interpolation|FInterpTo (Variables|/Script/Engine.CameraComponent|GetOrthoWidth _camera) (Math|Float|Max(Float) (+ (Math|Float|Max(Float) _y _x) (Variables|Default|GetBoundViewPadding)) (Variables|Default|GetMinimumProjectionWidth)) Delta 1.0)))))

(event EventBeginPlay
  ;[0 0 0] Slow tick waiting wor hex tile actor to be spawned in the world for use with the normal  tick
  (CallFunction|StartSlowTick))

(event EventTick
  (params (DeltaSeconds :type Float%20%28single-precision%29))
  ;[1 0 0] Coemstic camera update tick event
  (CallFunction|TickCameraUpdate DeltaSeconds))

(event Input|MouseEvents|LeftMouseButton
  (params (Key :type Key%20Structure :default "None"))
  (bind _returnvalue (Game|GetPlayerController 0))
  (bind _worldlocation (Game|Player|ConvertMouseLocationToWorldSpace _returnvalue))
  (bind (_x _y) (Math|Vector|BreakVector _worldlocation))
  (bind (_x_2 _y_2) (Math|Vector|BreakVector _worldlocation))
  ;[1 1 1] Testing hex mesh instance identification and deletion
  (:Pressed
    (bind (_outhit _returnvalue_2) (Collision|LineTraceByChannel (Math|Vector|MakeVector _x _y 888888.0) (Math|Vector|MakeVector _x_2 _y_2 -888888.0) "TraceTypeQuery2" false 0 "ForDuration"))
    (if _returnvalue_2
      (bind _asinstanced_static_mesh_component (Utilities|Casting|CastToInstancedStaticMeshComponent (.HitComponent (Collision|BreakHitResult _outhit))))
      (if (.Success (CallFunction|GetClosestInstanceWorldSpace _asinstanced_static_mesh_component (.ImpactPoint (Collision|BreakHitResult _outhit)) 1e+01 false))
        (Development|PrintString (Utilities|String|ToString(Integer) (.InstanceIndex (CallFunction|GetClosestInstanceWorldSpace _asinstanced_static_mesh_component (.ImpactPoint (Collision|BreakHitResult _outhit)) 1e+01 false))))
        (Class|InstancedStaticMeshComponent|RemoveInstance _asinstanced_static_mesh_component (.InstanceIndex (CallFunction|GetClosestInstanceWorldSpace _asinstanced_static_mesh_component (.ImpactPoint (Collision|BreakHitResult _outhit)) 1e+01 false)))))))

(event Input|KeyboardEvents|SpaceBar
  (params (Key :type Key%20Structure :default "None"))
  (bind _hex (Utilities|Struct|MakeHex 3 4))
  (bind _hex_2 (Utilities|Struct|MakeHex 1 2))
  (bind _returnvalue (Class|BasicHexBlueprintFunctionLibrary|AddHexHex _hex_2 _hex))
  (bind (_q _r _s) (Utilities|Struct|BreakHex _returnvalue))
  ;[1 1 1] Just a test for custom operator overload nodes, Hex + Hex structure in this case
  (:Pressed
    (Development|PrintString "Hello")
    (Development|PrintString (Utilities|String|ToString(Integer) _q))
    (Development|PrintString (Utilities|String|ToString(Integer) _r))
    (Development|PrintString (Utilities|String|ToString(Integer) _s))
    (Development|PrintString "Bye")))

(fn ConstructionScript)

(fn GetClosestInstanceWorldSpace
  (params (InstancedStaticMeshComponent :type Instanced%20Static%20Mesh%20Component%20Object%20Reference) (Center :type Vector%20%28by%20ref%29) (Radius :type Float%20%28single-precision%29) (bSphereInWorldSpace :type Boolean))
  (LocalVariables|SetClosestDistance 9.223372036854776e+18)
  (LocalVariables|SetClosestIndex -1)
  (for _array_element (Class|InstancedStaticMeshComponent|GetInstancesOverlappingSphere InstancedStaticMeshComponent Center Radius bSphereInWorldSpace)
    (if (> (LocalVariables|GetClosestDistance) (Math|Vector|Distance(Vector) (.Location (Math|Transform|BreakTransform (.OutInstanceTransform (Components|InstancedStaticMesh|GetInstanceTransform InstancedStaticMeshComponent _array_element true)))) Center))
      (LocalVariables|SetClosestDistance (Math|Vector|Distance(Vector) (.Location (Math|Transform|BreakTransform (.OutInstanceTransform (Components|InstancedStaticMesh|GetInstanceTransform InstancedStaticMeshComponent _array_element true)))) Center))
      (LocalVariables|SetClosestIndex _array_element)))
  (return (>= (LocalVariables|GetClosestIndex) 0) (LocalVariables|GetClosestIndex)))